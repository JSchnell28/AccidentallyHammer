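; Character Blueprint that reacts to Chaos physics collisions on a geometry collection in the level.
; The construction script caches the GeometryCollectionActor found by class, and BeginPlay binds to its component's collision event.
; Each collision applies a small kinematic field at a fixed zero position, ignoring the impact location.
; A disconnected node that would spawn a FieldSystem at the collision location never runs.
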(event Custom|OnChaosPhysicsCollsion_Event_1
  (params (CollisionInfo :type Chaos%20Physics%20Collision%20Info%20Structure%20%28by%20ref%29))
  (Class|GeometryCollectionComponent|ApplyKinematicField (Variables|/Script/GeometryCollectionEngine.GeometryCollectionActor|GetGeometryCollectionComponent (Variables|Default|GetGeometryCollectionActor)) 2.0 "0, 0, 0"))

(event EventBeginPlay
  (EventDispatchers|BindEventtoOnChaosPhysicsCollision (Variables|/Script/GeometryCollectionEngine.GeometryCollectionActor|GetGeometryCollectionComponent (Variables|Default|GetGeometryCollectionActor)) (delegate Custom|OnChaosPhysicsCollsion_Event_1)))

(fn ConstructionScript
  (bind _returnvalue (Actor|GetActorOfClass "/Script/GeometryCollectionEngine.GeometryCollectionActor"))
  (Variables|Default|SetGeometryCollectionActor _returnvalue))